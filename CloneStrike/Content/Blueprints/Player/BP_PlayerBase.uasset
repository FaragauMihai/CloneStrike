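; BP_PlayerBase is a player base Blueprint that provides movement and mouse look through Enhanced Input.
; On BeginPlay it gets the player controller reference through a message call on its controller and adds the default mapping context.
; IA_Movement feeds movement input along the actor's forward and right vectors, while IA_Look drives controller yaw and pitch.
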(event `self.ReceiveBeginPlay`
  (bind _playercontroller (message `/Game/Blueprints/Interfaces/INT_PlayerController.GetPlayerControllerRef` (`self.GetController`)))
  (`EnhancedInputSubsystemInterface.AddMappingContext` (pcsubsystem `EnhancedInputLocalPlayerSubsystem` _playercontroller) "/Game/Blueprints/Player/Input/IMC_Default.IMC_Default" 0 (struct)))

(event `EnhancedInput|/Game/Blueprints/Player/Input/IA_Movement`
  (params (ActionValue :type "Vector2D Structure") (ElapsedSeconds :type "Float (double-precision)") (TriggeredSeconds :type "Float (double-precision)") (InputAction :type "InputAction Object Reference" :default "/Game/Blueprints/Player/Input/IA_Movement.IA_Movement"))
  ;[1 1 1] W/S/A/D Movement
  (:`Triggered`
    (`self.AddMovementInput` (`self.GetActorForwardVector`) ActionValue_X)
    (`self.AddMovementInput` (`self.GetActorRightVector`) ActionValue_Y)))

(event `EnhancedInput|/Game/Blueprints/Player/Input/IA_Look`
  (params (ActionValue :type "Vector2D Structure") (ElapsedSeconds :type "Float (double-precision)") (TriggeredSeconds :type "Float (double-precision)") (InputAction :type "InputAction Object Reference" :default "/Game/Blueprints/Player/Input/IA_Look.IA_Look"))
  ;[1 1 1] Mouse Look
  (:`Triggered`
    (`self.AddControllerYawInput` ActionValue_X)
    (`self.AddControllerPitchInput` ActionValue_Y)))

(fn `UserConstructionScript`)