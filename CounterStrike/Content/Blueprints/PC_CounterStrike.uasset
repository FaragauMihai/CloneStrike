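; Player controller for a Counter-Strike-style game that handles team selection and player spawning.
; On BeginPlay it shows the team selection widget through client events and caches the game mode via an interface message.
; Team choices go through a server event to the game mode's spawn request.
; SpawnPlayer spawns the chosen pawn class at the given transform, possesses it, and tells the client to hide the widget.
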(event `self.ReceiveBeginPlay`
  ;[1 1 1] Show Team Selection Widget
  (`self.ShowHideWidget` "NewEnumerator0" true)
  (bind _gamemode (message `/Game/Blueprints/Interfaces/INT_GameMode.GetGameModeRef` (`GameplayStatics.GetGameMode`)))
  (set `self.GameMode` _gamemode))

(event `ShowHideWidget`
  (params (Widgets :type "/Game/Blueprints/Enums/E_GameWidgets Enum" :default "NewEnumerator0") (bShow :type Boolean))
  ;[1 1 1] Show Team Selection Widget
  (`self.CL_ShowHideWidget` Widgets bShow))

(event `CL_ShowHideWidget`
  (params (Widget :type "/Game/Blueprints/Enums/E_GameWidgets Enum" :default "NewEnumerator0") (bShow :type Boolean))
  ;[1 1 1] Show Team Selection Widget
  (if bShow
    (`self.f_ShowWidget` Widget)
    (else
      (`self.f_HideWidget` Widget))))

(event `SelectTeam`
  (params (Team :type "Actor Class Reference"))
  (`self.SRV_SelectTeam` Team))

(event `SRV_SelectTeam`
  (params (Team :type "Actor Class Reference"))
  (`/Game/Blueprints/GM_CounterStrike.RequestSpawnPlayer` (`self.GameMode`) self Team))

(event `SpawnPlayer`
  (params (Team :type "Actor Class Reference") (SpawnTransform :type "Transform Structure"))
  (bind _returnvalue (`|SpawnActorFromClass` Team SpawnTransform "AdjustIfPossibleButAlwaysSpawn" "MultiplyWithRoot" null null))
  (bind _output_get (set `self.PlayerPawn` _returnvalue))
  (bind _player (message `/Game/Blueprints/Interfaces/INT_PlayerBase.GetPlayerRef` _output_get))
  (`self.Possess` _player)
  (`self.CL_SpawnPlayer`))

(event `CL_SpawnPlayer`
  (`self.ShowHideWidget` "NewEnumerator0"))

(fn `f_HideWidget`
  (params (Widget :type "/Game/Blueprints/Enums/E_GameWidgets Enum" :default "NewEnumerator0"))
  (switch `/Game/Blueprints/Enums/E_GameWidgets` Widget
    (:`NewEnumerator0`
      (bind _wb_teamselection (`self.WB_TeamSelection`)
        (:`then`
          (`Widget.RemoveFromParent` _wb_teamselection))
        (:`else`)))))

(fn `f_ShowWidget`
  (params (Widget :type "/Game/Blueprints/Enums/E_GameWidgets Enum" :default "NewEnumerator0"))
  (switch `/Game/Blueprints/Enums/E_GameWidgets` Widget
    (:`NewEnumerator0`
      (`self.WB_TeamSelection`
        (:`then`
          _)
        (:`else`
          (bind _returnvalue (`|CreateWidget` "/Game/UI/WB_TeamSelection.WB_TeamSelection_C"))
          (bind _output_get (set `self.WB_TeamSelection` _returnvalue))))
      (`UserWidget.AddToViewport` _output_get 0))))

(fn `GetPlayerControllerRef`
  (returns (PlayerController :type "/Game/Blueprints/PC_CounterStrike Object Reference"))
  (return self))

(fn `UserConstructionScript`)