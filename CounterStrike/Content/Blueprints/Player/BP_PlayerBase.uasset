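; Base multiplayer player character with Enhanced Input movement, looking, crouching, walking, jumping, and weapon looting, swapping and dropping.
; A movement-state stack sets speed, with changes and aim pitch relayed to the server; running triggers timed, multicast footstep sounds.
; Overlapped weapons queue into a server-side inventory.
; OnRep handlers attach looted weapons to hand, thigh or back sockets and detach dropped ones with physics enabled.
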(event `self.ReceiveBeginPlay`
  (`KismetSystemLibrary.Delay` 0.05)
  (bind _playercontroller (message `/Game/Blueprints/Interfaces/INT_PlayerController.GetPlayerControllerRef` (`self.GetController`)))
  (`/Engine/EditorBlueprintResources/StandardMacros.IsValid` _playercontroller
    (:`Is Valid`
      (bind _returnvalue (pcsubsystem `EnhancedInputLocalPlayerSubsystem` _playercontroller))
      (`/Engine/EditorBlueprintResources/StandardMacros.IsValid` _returnvalue
        (:`Is Valid`
          (`EnhancedInputSubsystemInterface.AddMappingContext` _returnvalue "/Game/Blueprints/Player/Input/IMC_Default.IMC_Default" 0 (struct))
          (`SkinnedMeshComponent.HideBoneByName` (`self.Mesh`) "head" "PBO_None"))))))

(event `EnhancedInput|/Game/Blueprints/Player/Input/IA_Movement`
  (params (ActionValue :type "Vector2D Structure") (ElapsedSeconds :type "Float (double-precision)") (TriggeredSeconds :type "Float (double-precision)") (InputAction :type "InputAction Object Reference" :default "/Game/Blueprints/Player/Input/IA_Movement.IA_Movement"))
  (bind _x (.x (`self.GetVelocity`)))
  (bind _y (.y (`self.GetVelocity`)))
  ;[1 1 1] WASD Movement
  (:`Triggered`
    (`self.AddMovementInput` (`self.GetActorForwardVector`) ActionValue_X)
    (`self.AddMovementInput` (`self.GetActorRightVector`) ActionValue_Y)
    (if (and (or (> _x 250.0) (< _x -250.0) (> _y 250.0) (< _y -250.0) false) (`self.f_IsNotJumping`) (`self.f_IsRunning`) (> TriggeredSeconds 0.3))
      (if (not (`self.PlayingFootstepsSFX`))
        (`self.SRV_PlayFootstepsSFX`)
        (set `self.PlayingFootstepsSFX` true)
        (bind _returnvalue (`KismetSystemLibrary.K2_SetTimerDelegate` (delegate `PlayFootstepsSFX`) 0.42 true))
        (set `self.FootstepsSFXTimerHandle` _returnvalue))
      (else
        (if (`KismetSystemLibrary.K2_IsValidTimerHandle` (`self.FootstepsSFXTimerHandle`)) :!label _label
          (`KismetSystemLibrary.K2_ClearAndInvalidateTimerHandle` (`self.FootstepsSFXTimerHandle`))
          (set `self.PlayingFootstepsSFX` false)))))
  (:`Completed`
    (goto _label)))

(event `PlayFootstepsSFX`
  ;[1 1 1] WASD Movement
  (`self.SRV_PlayFootstepsSFX`))

(event `SRV_PlayFootstepsSFX`
  ;[1 1 1] WASD Movement
  (`self.MC_PlayFootstepsSFX`))

(event `MC_PlayFootstepsSFX`
  ;[1 1 1] WASD Movement
  (`GameplayStatics.PlaySoundAtLocation` "/Game/Audio/SFX/SC_Footsteps.SC_Footsteps" (`self.K2_GetActorLocation`) (struct) 1.0 1.0 0.0 null null null null))

(event `EnhancedInput|/Game/Blueprints/Player/Input/IA_Look`
  (params (ActionValue :type "Vector2D Structure") (ElapsedSeconds :type "Float (double-precision)") (TriggeredSeconds :type "Float (double-precision)") (InputAction :type "InputAction Object Reference" :default "/Game/Blueprints/Player/Input/IA_Look.IA_Look"))
  ;[1 1 1] Mouse Looking
  (:`Triggered`
    (`self.AddControllerYawInput` ActionValue_X)
    (`self.AddControllerPitchInput` ActionValue_Y)
    (`self.f_CalculateAimDirection`)))

(event `SRV_CalculateAimDIrection`
  ;[1 1 1] Mouse Looking
  (`self.f_CalculateAimDirection`))

(event `EnhancedInput|/Game/Blueprints/Player/Input/IA_Crouch`
  (params (ActionValue :type Boolean) (ElapsedSeconds :type "Float (double-precision)") (TriggeredSeconds :type "Float (double-precision)") (InputAction :type "InputAction Object Reference" :default "/Game/Blueprints/Player/Input/IA_Crouch.IA_Crouch"))
  ;[1 1 1] Crouch Movement
  (:`Triggered`
    (if (`self.f_IsNotJumping`) :!label _label_2
      (if ActionValue
        (`self.f_Crouch` true)
        (elif (`KismetArrayLibrary.Array_Contains` (`self.MovementState`) "NewEnumerator2")
          (`self.f_Crouch` false)))
      (else
        (`KismetSystemLibrary.Delay` 0.05)
        (goto _label_2)))))

(event `SRV_Crouch`
  (params (bCrouch :type Boolean))
  ;[1 1 1] Crouch Movement
  (`self.f_Crouch` bCrouch))

(event `EnhancedInput|/Game/Blueprints/Player/Input/IA_Walk`
  (params (ActionValue :type Boolean) (ElapsedSeconds :type "Float (double-precision)") (TriggeredSeconds :type "Float (double-precision)") (InputAction :type "InputAction Object Reference" :default "/Game/Blueprints/Player/Input/IA_Walk.IA_Walk"))
  ;[1 1 1] Walk Movement
  (:`Triggered`
    (if ActionValue
      (`self.f_Walk` true)
      (else
        (`self.f_Walk` false)))))

(event `SRV_Walk`
  (params (bWalk :type Boolean))
  ;[1 1 1] Walk Movement
  (`self.f_Walk` bWalk))

(event `EnhancedInput|/Game/Blueprints/Player/Input/IA_Jump`
  (params (ActionValue :type Boolean) (ElapsedSeconds :type "Float (double-precision)") (TriggeredSeconds :type "Float (double-precision)") (InputAction :type "InputAction Object Reference" :default "/Game/Blueprints/Player/Input/IA_Jump.IA_Jump"))
  ;[1 1 1] Jumping
  (:`Triggered`
    (if (`self.f_IsNotJumping`)
      (`self.Jump`))))

(event `AddOverlappedWeapons`
  (params (Weapon :type "/Game/Blueprints/Weapons/BP_WeaponBase Object Reference"))
  (`self.SRV_AddOverlappedWeapons` Weapon))

(event `CheckForOverlappedWeapon`
  (`self.LootWeapon` :!label _label_3))

(event `SRV_AddOverlappedWeapons`
  (params (Weapon :type "/Game/Blueprints/Weapons/BP_WeaponBase Object Reference"))
  (bind _overlappedweapons (`self.OverlappedWeapons`))
  (`KismetArrayLibrary.Array_Set` _overlappedweapons (`KismetArrayLibrary.Array_Length` _overlappedweapons) Weapon true)
  (`/Engine/EditorBlueprintResources/StandardMacros.DoOnce` false :!label _label_4
    (:`Completed`
      (goto _label_3))))

(event `CanLootWeaponAgain`
  (goto _label_4 :!via `Reset`))

(event `LootWeapon`
  ;[1 1 1] Loot Weapon Logic
  (`self.SRV_LootWeapon`))

(event `SRV_LootWeapon`
  (bind _weaponinventory (`self.WeaponInventory`))
  (bind _overlappedweapons (`self.OverlappedWeapons`))
  (bind _output (`|GetArrayItem` _overlappedweapons))
  (bind (_weaponinfo_name _weaponinfo_type) (break `/Game/Blueprints/Structs/ST_WeaponInfo` (`/Game/Blueprints/Libraries/BP_FunctionLibrary.f_GetWeaponInfo` (`/Game/Blueprints/Weapons/BP_WeaponBase.WeaponName` (`self.LootedWeapon`)))))
  ;[1 1 1] Loot Weapon Logic
  (if (`KismetArrayLibrary.Array_IsNotEmpty` _overlappedweapons)
    (`KismetArrayLibrary.Array_Set` _weaponinventory (`KismetArrayLibrary.Array_Length` _weaponinventory) _output true)
    (set `self.LootedWeapon` _output)
    (if (`|EnumEquality` (`self.EquippedWeaponType`) "NewEnumerator2")
      ;;[0.07292 0.0302 0 1 10] Makes sure that the weapon attached to the hand before changing player equpped weapon state
      ;; 8.12 Attaching Weapons to Back
      (`KismetSystemLibrary.Delay` 0.05)
      (`self.SetEquippedWeaponType` _weaponinfo_type))
    (`KismetArrayLibrary.Array_RemoveItem` (`self.OverlappedWeapons`) _output)
    (`self.CheckForOverlappedWeapon`)
    (else
      (`self.CanLootWeaponAgain`)
      (`KismetSystemLibrary.Delay` 0.1)
      (set `self.LootedWeapon` null))))

(event `SetEquippedWeaponType`
  (params (EquippedWeaponType :type "/Game/Blueprints/Enums/E_WeaponType Enum" :default "NewEnumerator2"))
  ;[1 1 1] Loot Weapon Logic
  (`self.SRV_SetEquippedWeapon` EquippedWeaponType))

(event `SRV_SetEquippedWeapon`
  (params (EquippedWeaponType :type "/Game/Blueprints/Enums/E_WeaponType Enum" :default "NewEnumerator2"))
  ;[1 1 1] Loot Weapon Logic
  (set `self.EquippedWeaponType` EquippedWeaponType))

(event `EnhancedInput|/Game/Blueprints/Player/Input/IA_DropWeapon`
  (params (ActionValue :type Boolean) (ElapsedSeconds :type "Float (double-precision)") (TriggeredSeconds :type "Float (double-precision)") (InputAction :type "InputAction Object Reference" :default "/Game/Blueprints/Player/Input/IA_DropWeapon.IA_DropWeapon"))
  (:`Triggered`
    (if (`|EnumInequality` (`self.EquippedWeaponType`) "NewEnumerator2")
      (`self.SRV_DropWeaponTYpe`))))

(event `SRV_DropWeaponType`
  (for _array_element (`self.WeaponInventory`)
    (bind (_weaponinfo_name _weaponinfo_type) (break `/Game/Blueprints/Structs/ST_WeaponInfo` (`/Game/Blueprints/Libraries/BP_FunctionLibrary.f_GetWeaponInfo` (`/Game/Blueprints/Weapons/BP_WeaponBase.WeaponName` _array_element))))
    (if (`|EnumEquality` _weaponinfo_type (`self.EquippedWeaponType`))
      (`self.f_DropWeapon` _array_element)
      (break)))
  (`KismetSystemLibrary.Delay` 0.1)
  (set `/Game/Blueprints/Weapons/BP_WeaponBase.bCanBeInteractedWith` true (`self.WeaponToDrop`))
  (set `self.WeaponToDrop` null))

(event `SetDroppedWeapon`
  (params (DroppedWeapon :type "/Game/Blueprints/Weapons/BP_WeaponBase Object Reference"))
  (`self.SRV_SetDroppedWeapon` DroppedWeapon))

(event `SRV_SetDroppedWeapon`
  (params (DroppedWeapon :type "/Game/Blueprints/Weapons/BP_WeaponBase Object Reference"))
  (set `self.DroppedWeapon` DroppedWeapon))

(event `EnhancedInput|/Game/Blueprints/Player/Input/IA_LootWeapon`
  (params (ActionValue :type Boolean) (ElapsedSeconds :type "Float (double-precision)") (TriggeredSeconds :type "Float (double-precision)") (InputAction :type "InputAction Object Reference" :default "/Game/Blueprints/Player/Input/IA_LootWeapon.IA_LootWeapon"))
  (:`Triggered`
    (`self.SRV_RequesteLootWeapon`)))

(event `SRV_RequesteLootWeapon`
  (bind _overlappingactors (`self.GetOverlappingActors` "/Game/Blueprints/Weapons/BP_WeaponBase.BP_WeaponBase_C"))
  (if (`KismetArrayLibrary.Array_IsNotEmpty` _overlappingactors)
    (for _array_element (`self.WeaponInventory`)
      (bind _weapon (message `/Game/Blueprints/Interfaces/INT_WeaponBase.GetWeapon Ref` (`|GetArrayItem` _overlappingactors)))
      (bind (_weaponinfo_name _weaponinfo_type) (break `/Game/Blueprints/Structs/ST_WeaponInfo` (`/Game/Blueprints/Libraries/BP_FunctionLibrary.f_GetWeaponInfo` (`/Game/Blueprints/Weapons/BP_WeaponBase.WeaponName` _array_element))))
      (bind (_weaponinfo_name_2 _weaponinfo_type_2) (break `/Game/Blueprints/Structs/ST_WeaponInfo` (`/Game/Blueprints/Libraries/BP_FunctionLibrary.f_GetWeaponInfo` (`/Game/Blueprints/Weapons/BP_WeaponBase.WeaponName` _weapon))))
      (if (`|EnumEquality` _weaponinfo_type _weaponinfo_type_2)
        (`self.f_DropWeapon` _array_element)
        (`self.AddOverlappedWeapons` _weapon)
        (break)))
    (`KismetSystemLibrary.Delay` 0.1)
    (set `/Game/Blueprints/Weapons/BP_WeaponBase.bCanBeInteractedWith` true (`self.WeaponToDrop`))
    (set `self.WeaponToDrop` null)))

(fn `f_CalculateAimDirection`
  (bind (_returnvalue_roll _returnvalue_pitch) (`KismetMathLibrary.BreakRotator` (`KismetMathLibrary.NormalizedDeltaRotator` (`self.GetControlRotation`) (`self.K2_GetActorRotation`))))
  (`/Engine/EditorBlueprintResources/ActorMacros.Switch Has Authority`
    (:`Authority`
      _)
    (:`Remote`
      (`self.SRV_CalculateAimDIrection`)))
  (set `self.AimDirection` _returnvalue_pitch))

(fn `f_Crouch`
  (params (bCrouch :type Boolean))
  (locals (CrouchLocal :type Boolean))
  (bind _movementstate (`self.MovementState`))
  (bind _output_get (set `local.CrouchLocal` bCrouch))
  (`/Engine/EditorBlueprintResources/ActorMacros.Switch Has Authority`
    (:`Authority`
      _)
    (:`Remote`
      (`self.SRV_Crouch` _output_get)))
  (if (`local.CrouchLocal`)
    (`self.Crouch`)
    (`KismetArrayLibrary.Array_Set` _movementstate (+ (`KismetArrayLibrary.Array_LastIndex` _movementstate) 1) "NewEnumerator2" true)
    (`self.f_SetMovementSpeed`)
    (else
      (`self.UnCrouch`)
      (`KismetArrayLibrary.Array_RemoveItem` (`self.MovementState`) "NewEnumerator2")
      (`self.f_SetMovementSpeed`))))

(fn `f_DropWeapon`
  (params (WeaponToDrop :type "/Game/Blueprints/Weapons/BP_WeaponBase Object Reference"))
  (set `/Game/Blueprints/Weapons/BP_WeaponBase.bCanBeInteractedWith` false WeaponToDrop)
  (bind _output_get (set `self.WeaponToDrop` WeaponToDrop))
  (`self.SetDroppedWeapon` _output_get)
  (`KismetArrayLibrary.Array_RemoveItem` (`self.WeaponInventory`) WeaponToDrop)
  (bind (_weaponinfo_name _weaponinfo_type) (break `/Game/Blueprints/Structs/ST_WeaponInfo` (`/Game/Blueprints/Libraries/BP_FunctionLibrary.f_GetWeaponInfo` (`/Game/Blueprints/Weapons/BP_WeaponBase.WeaponName` _output_get))))
  (if (`|EnumEquality` (`self.EquippedWeaponType`) _weaponinfo_type)
    (`self.SetEquippedWeaponType` "NewEnumerator2")))

(fn `f_IsNotJumping`
  (returns (ReturnValue :type Boolean))
  (return (not (`NavMovementComponent.IsFalling` (`self.CharacterMovement`)))))

(fn `f_IsRunning`
  (returns (ReturnValue :type Boolean))
  (bind _movementstate (`self.MovementState`))
  (return (`|EnumEquality` (`|GetArrayItem` _movementstate (`KismetArrayLibrary.Array_LastIndex` _movementstate)) "NewEnumerator0")))

(fn `f_SetMovementSpeed`
  (bind _movementstate (`self.MovementState`))
  (bind _movementstate_2 (`self.MovementState`))
  (if (`|EnumEquality` (`|GetArrayItem` _movementstate (`KismetArrayLibrary.Array_LastIndex` _movementstate)) "NewEnumerator2")
    (`self.Crouch`)
    (else
      (`self.UnCrouch`)))
  (set `CharacterMovementComponent.MaxWalkSpeed` (select `/Game/Blueprints/Enums/E_MovementStates` (`|GetArrayItem` _movementstate_2 (`KismetArrayLibrary.Array_LastIndex` _movementstate_2)) :`NewEnumerator0` (`self.RunSpeed`) :`NewEnumerator1` (`self.WalkSpeed`) :`NewEnumerator2` (`self.CrouchSpeed`)) (`self.CharacterMovement`)))

(fn `f_Walk`
  (params (bWalk :type Boolean))
  (locals (WalkLocal :type Boolean))
  (bind _movementstate (`self.MovementState`))
  (bind _output_get (set `local.WalkLocal` bWalk))
  (`/Engine/EditorBlueprintResources/ActorMacros.Switch Has Authority`
    (:`Authority`
      _)
    (:`Remote`
      (`self.SRV_Walk` _output_get)))
  (if (`local.WalkLocal`)
    (`KismetArrayLibrary.Array_Set` _movementstate (+ (`KismetArrayLibrary.Array_LastIndex` _movementstate) 1) "NewEnumerator1" true)
    (`self.f_SetMovementSpeed`)
    (else
      (`KismetArrayLibrary.Array_RemoveItem` (`self.MovementState`) "NewEnumerator1")
      (`self.f_SetMovementSpeed`))))

(fn `GetPlayerRef`
  (returns (Player :type "/Game/Blueprints/Player/BP_PlayerBase Object Reference"))
  (return self))

(fn `OnRep_LootedWeapon`
  (bind _lootedweapon (`self.LootedWeapon`))
  (bind _weapon (`/Game/Blueprints/Weapons/BP_WeaponBase.Weapon` _lootedweapon))
  (bind (_weaponinfo_name _weaponinfo_type) (break `/Game/Blueprints/Structs/ST_WeaponInfo` (`/Game/Blueprints/Libraries/BP_FunctionLibrary.f_GetWeaponInfo` (`/Game/Blueprints/Weapons/BP_WeaponBase.WeaponName` (`self.LootedWeapon`)))))
  (bind (_weaponinfo_name_2 _weaponinfo_type_2) (break `/Game/Blueprints/Structs/ST_WeaponInfo` (`/Game/Blueprints/Libraries/BP_FunctionLibrary.f_GetWeaponInfo` (`/Game/Blueprints/Weapons/BP_WeaponBase.WeaponName` (`self.LootedWeapon`)))))
  (bind _lootedweapon_2 (`self.LootedWeapon`)
    (:`then`
      (bind _weapon_2 (`/Game/Blueprints/Weapons/BP_WeaponBase.Weapon` _lootedweapon_2))
      (`PrimitiveComponent.SetSimulatePhysics` _weapon_2 false)
      (`PrimitiveComponent.SetCollisionEnabled` _weapon_2 "NoCollision")
      (`PrimitiveComponent.SetCollisionEnabled` (`/Game/Blueprints/Weapons/BP_WeaponBase.CollisionSphere` (`self.LootedWeapon`)) "NoCollision")
      (`SceneComponent.K2_AttachToComponent` _weapon (`/Game/Blueprints/Weapons/BP_WeaponBase.DefaultSceneRoot` _lootedweapon) "None" "SnapToTarget" "SnapToTarget" "SnapToTarget" true)
      (`SceneComponent.ResetRelativeTransform` _weapon)
      (if (`|EnumEquality` (`self.EquippedWeaponType`) "NewEnumerator2")
        (`self.K2_AttachToComponent` (`self.LootedWeapon`) (`self.Mesh`) (select `/Game/Blueprints/Enums/E_WeaponType` _weaponinfo_type_2 :`NewEnumerator1` "S_Pistol" :`NewEnumerator0` "S_Rifle" :!type "Name") "SnapToTarget" "SnapToTarget" "SnapToTarget" true)
        (else
          (`self.K2_AttachToComponent` (`self.LootedWeapon`) (`self.Mesh`) (select `/Game/Blueprints/Enums/E_WeaponType` _weaponinfo_type :`NewEnumerator1` "S_Weapon_Thigh" :`NewEnumerator0` "S_Weapon_Back" :!type "Name") "SnapToTarget" "SnapToTarget" "SnapToTarget" true))))
    (:`else`)))

(fn `OnRep_WeaponToDrop`
  (bind _weapon (`/Game/Blueprints/Weapons/BP_WeaponBase.Weapon` (`self.WeaponToDrop`)))
  (bind _weapontodrop (`self.WeaponToDrop`)
    (:`then`
      (`self.K2_DetachFromActor` _weapontodrop "KeepWorld" "KeepWorld" "KeepWorld")
      (`PrimitiveComponent.SetCollisionEnabled` _weapon "PhysicsOnly")
      (`PrimitiveComponent.SetSimulatePhysics` _weapon true)
      (`PrimitiveComponent.SetCollisionEnabled` (`/Game/Blueprints/Weapons/BP_WeaponBase.CollisionSphere` (`self.WeaponToDrop`)) "QueryOnly"))
    (:`else`)))

(fn `UserConstructionScript`)